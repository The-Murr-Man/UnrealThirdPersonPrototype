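; Health pickup actor that heals the shooter character when it overlaps the pickup's sphere.
; On overlap it casts to BP_ShooterCharacter and adds HealingAmount to Health, capped at MaxHealth.
; A successful heal plays a pickup sound at the actor's location and destroys the pickup.
; At full health it only prints a debug message and stays in the world.
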(event `self.Sphere.OnComponentBeginOverlap`
  (params (OverlappedComponent :type "PrimitiveComponent Object Reference") (OtherActor :type "Actor Object Reference") (OtherComp :type "PrimitiveComponent Object Reference") (OtherBodyIndex :type Integer) (bFromSweep :type Boolean) (SweepResult :type "HitResult Structure (by ref)"))
  (bind _asbp_shooter_character (cast `/Game/_Game/BPs/Character/BP_ShooterCharacter` OtherActor))
  (bind _health (`ShooterCharacter.health` _asbp_shooter_character))
  (if (== _health (`ShooterCharacter.maxHealth` _asbp_shooter_character))
    (`KismetSystemLibrary.PrintString` "Full")
    (else
      (bind _returnvalue (+ _health (`self.HealingAmount`)))
      (bind _maxhealth (`ShooterCharacter.maxHealth` _asbp_shooter_character))
      (if (> _returnvalue _maxhealth)
        (set `ShooterCharacter.health` _maxhealth _asbp_shooter_character)
        (else
          (set `ShooterCharacter.health` _returnvalue _asbp_shooter_character)))
      (`GameplayStatics.PlaySoundAtLocation` (`self.HealthPickupSound`) (`self.K2_GetActorLocation`) (struct) 1.0 1.0 0.0 null null null)
      (`self.K2_DestroyActor` self))))

(fn `UserConstructionScript`)
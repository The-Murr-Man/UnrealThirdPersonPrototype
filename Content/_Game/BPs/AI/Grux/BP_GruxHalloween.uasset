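; BP_GruxHalloween is a Halloween Grux enemy that adds health bar and floating damage number UI to its parent class.
; On BeginPlay it binds itself to its WBP_EnemyHealthBar widget and hides it, with show and hide events toggling visibility.
; ShowDamageNumber spawns a WBP_DamageNumber at the projected hit location, passes it to StoreDamageNumber, sets damage and headshot data, then plays its animation.
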(event `self.ReceiveBeginPlay`
  (bind _healthbar (`self.HealthBar`))
  (`parent.ReceiveBeginPlay`)
  (bind _aswbp_enemy_health_bar (cast `/Game/_Game/HUD/WBP_EnemyHealthBar` (`WidgetComponent.GetUserWidgetObject` _healthbar)))
  (set `/Game/_Game/HUD/WBP_EnemyHealthBar.Enemy` self _aswbp_enemy_health_bar)
  (`Widget.SetVisibility` (`WidgetComponent.GetUserWidgetObject` _healthbar) "Hidden"))

(event `self.ShowHealthBar`
  (`Widget.SetVisibility` (`WidgetComponent.GetUserWidgetObject` (`self.HealthBar`)) "Visible")
  (`parent.ShowHealthBar`))

(event `self.HideHealthBar`
  (`Widget.SetVisibility` (`WidgetComponent.GetUserWidgetObject` (`self.HealthBar`)) "Hidden"))

(event `self.ShowDamageNumber`
  (params (damage :type Integer) (hitLocation :type "Vector Structure") (bIsHeadShot :type Boolean))
  (bind _returnvalue (`|CreateWidget` "/Game/_Game/HUD/WBP_DamageNumber.WBP_DamageNumber_C"))
  (`UserWidget.AddToViewport` _returnvalue 0)
  (`UserWidget.SetPositionInViewport` _returnvalue (`GameplayStatics.ProjectWorldToScreen` (`GameplayStatics.GetPlayerController` 0) hitLocation) true)
  (`self.StoreDamageNumber` _returnvalue hitLocation)
  (set `/Game/_Game/HUD/WBP_DamageNumber.DamageText` (`KismetTextLibrary.Conv_IntToText` damage) _returnvalue)
  (set `/Game/_Game/HUD/WBP_DamageNumber.IsHeadShot` bIsHeadShot _returnvalue)
  (`UserWidget.PlayAnimation` _returnvalue (`/Game/_Game/HUD/WBP_DamageNumber.DamageNumberAnim` _returnvalue) 0.0 1 "Forward" 1.0 false))

(fn `UserConstructionScript`)